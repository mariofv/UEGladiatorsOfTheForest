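; Behavior tree task that, despite its Find Nearest Enemy name, picks a random reachable wander point around the AI's controlled pawn.
; It queries the navmesh within a configurable radius of the pawn, writes the point to the MoveToLocation blackboard key and finishes successfully.
; It fails when no point is found, and never calls FinishExecute if the pawn is invalid.
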(event `self.ReceiveExecuteAI`
  (params (OwnerController :type "AIController Object Reference") (ControlledPawn :type "Pawn Object Reference"))
  (bind (_randomlocation _returnvalue) (`NavigationSystemV1.K2_GetRandomReachablePointInRadius` (`Actor.K2_GetActorLocation` ControlledPawn) (`self.Radius`) null null))
  (`/Engine/EditorBlueprintResources/StandardMacros.IsValid` ControlledPawn
    (:`Is Valid`
      (if _returnvalue
        (set `self.Location` _randomlocation)
        (`BTFunctionLibrary.SetBlackboardValueAsVector` (`self.MoveToLocation`) (`self.Location`))
        (`self.FinishExecute` true)
        (else
          (`self.FinishExecute` false))))))