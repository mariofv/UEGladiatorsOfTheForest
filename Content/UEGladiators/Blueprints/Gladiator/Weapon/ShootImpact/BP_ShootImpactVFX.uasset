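; BP_ShootImpactVFX is an actor that plays the particle effect for a weapon shot impact.
; SpawnImpact picks the blood or concrete template and matching relative rotation from the impact type, then activates its ParticleSystem component.
; It flags IsAlive for one second and then clears it, without destroying the actor.
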(event `Event Spawn Impact`
  (params (ImpactType :type "WeaponShootImpactType Enum" :default "Blood"))
  (`ParticleSystemComponent.SetTemplate` (`self.ParticleSystem`) (select `WeaponShootImpactType` ImpactType :`Blood` "/Game/Realistic_Starter_VFX_Pack_Vol2/Particles/Blood/P_Blood_Splat_Cone.P_Blood_Splat_Cone" :`Concrete` "/Game/Realistic_Starter_VFX_Pack_Vol2/Particles/Hit/P_Asphalt.P_Asphalt" :!type "ParticleSystem Object Reference"))
  (`SceneComponent.K2_SetRelativeRotation` (`self.ParticleSystem`) (select `WeaponShootImpactType` ImpactType :`Blood` (struct :`Pitch` 90.0 :`Yaw` 180.0) :!type "Rotator Structure") false false)
  (`ActorComponent.Activate` (`self.ParticleSystem`) false)
  (set `self.IsAlive` true)
  (`KismetSystemLibrary.Delay` 1.0)
  (set `self.IsAlive` false))

(fn `UserConstructionScript`)