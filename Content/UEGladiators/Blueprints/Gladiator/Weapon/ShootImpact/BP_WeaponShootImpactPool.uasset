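; BP_WeaponShootImpactPool is an actor that pools impact effects for weapon shots.
; On BeginPlay it pre-spawns BP_ShootImpactVFX actors at its own transform, with the count driven by PoolSize.
; SpawnImpact loops through the pool without breaking, moving every actor not marked IsAlive to the given location and rotation and triggering its impact event with the given type.
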(event `self.ReceiveBeginPlay`
  (for _ (range (+ (`self.PoolSize`) 1))
    (bind _returnvalue (`|SpawnActorFromClass` "/Game/UEGladiators/Blueprints/Gladiator/Weapon/ShootImpact/BP_ShootImpactVFX.BP_ShootImpactVFX_C" (`self.GetTransform`) "Undefined" "OverrideRootScale" null null))
    (`KismetArrayLibrary.Array_Add` (`self.ImpactVFXPool`) _returnvalue)))

(event `self.SpawnImpact`
  (params (p_ImpactType :type "WeaponShootImpactType Enum" :default "Blood") (p_ImpactLocation :type "Vector Structure (by ref)") (p_ImpactDirection :type "Rotator Structure (by ref)"))
  (for _array_element (`self.ImpactVFXPool`)
    (if (not (`/Game/UEGladiators/Blueprints/Gladiator/Weapon/ShootImpact/BP_ShootImpactVFX.IsAlive` _array_element))
      (`self.K2_SetActorLocation` _array_element p_ImpactLocation false false)
      (`self.K2_SetActorRotation` _array_element p_ImpactDirection false)
      (`/Game/UEGladiators/Blueprints/Gladiator/Weapon/ShootImpact/BP_ShootImpactVFX.Event Spawn Impact` _array_element p_ImpactType))))

(fn `UserConstructionScript`)